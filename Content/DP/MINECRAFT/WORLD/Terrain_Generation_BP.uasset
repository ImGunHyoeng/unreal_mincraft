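; Minecraft-style terrain actor that builds a blocky landscape and lets the player place blocks on it.
; The Construction Script fills a Width by Length grid with Grass and Dirt instances, using three summed sine layers for rounded heights, with Dirt below zero.
; Left click traces from the active first or third person camera and adds the character's selected block at the grid-snapped hit point.
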(event EventBeginPlay
  (Input|EnableInput (Game|GetPlayerController 0))
  (bind _asbp_third_person_character (Utilities|Casting|CastToBP_ThirdPersonCharacter (Game|GetPlayerCharacter 0)))
  (Variables|Default|SetAs%20BP%20Third%20Person%20Character _asbp_third_person_character))

(event Collision|EventActorBeginOverlap
  (params (OtherActor :type Actor%20Object%20Reference)))

(event EventTick
  (params (DeltaSeconds :type Float%20%28single-precision%29)))

(event Input|MouseEvents|LeftMouseButton
  (params (Key :type Key%20Structure :default "None"))
  (bind _dirt (Variables|Default|GetDirt))
  (bind _as_bp_third_person_character (Variables|Default|GetAs%20BP%20Third%20Person%20Character))
  (bind _tile_size (Variables|Default|GetTile%20Size))
  (bind _grass (Variables|Default|GetGrass))
  (bind _dirt_2 (Variables|Default|GetDirt))
  (bind _as_bp_third_person_character_2 (Variables|Default|GetAs%20BP%20Third%20Person%20Character))
  (bind _grass_2 (Variables|Default|GetGrass))
  (bind _tile_size_2 (Variables|Default|GetTile%20Size))
  (bind _as_bp_third_person_character_3 (Variables|Default|GetAs%20BP%20Third%20Person%20Character))
  (bind _as_bp_third_person_character_4 (Variables|Default|GetAs%20BP%20Third%20Person%20Character))
  (bind _thirdpersoncamara (Variables|/Game/DP/MINECRAFT/PLAYER/BP_ThirdPersonCharacter.BP_ThirdPersonCharacter_C|GetThirdPersonCamara _as_bp_third_person_character_4))
  (bind _select_int (Variables|/Game/DP/MINECRAFT/PLAYER/BP_ThirdPersonCharacter.BP_ThirdPersonCharacter_C|Getselect%20int _as_bp_third_person_character_2))
  (bind _firstpersoncamara (Variables|/Game/DP/MINECRAFT/PLAYER/BP_ThirdPersonCharacter.BP_ThirdPersonCharacter_C|GetFirstPersonCamara _as_bp_third_person_character))
  (bind _select_int_2 (Variables|/Game/DP/MINECRAFT/PLAYER/BP_ThirdPersonCharacter.BP_ThirdPersonCharacter_C|Getselect%20int _as_bp_third_person_character_3))
  (bind _returnvalue (Transformation|GetWorldLocation _firstpersoncamara))
  (bind _returnvalue_2 (Transformation|GetWorldLocation _thirdpersoncamara))
  (bind _returnvalue_3 (Utilities|Select :Index _select_int_2 :Option%200 _grass_2 :Option%201 _dirt))
  (bind _returnvalue_4 (Utilities|Select :Index _select_int :Option%200 _grass :Option%201 _dirt_2))
  (:Pressed
    (if (Variables|/Game/DP/MINECRAFT/PLAYER/BP_ThirdPersonCharacter.BP_ThirdPersonCharacter_C|Getthird (Variables|Default|GetAs%20BP%20Third%20Person%20Character))
      (bind _outhit (Collision|LineTraceByChannel _returnvalue_2 (+ _returnvalue_2 (* (Math|Vector|GetForwardVector _thirdpersoncamara) (Variables|Default|Get1000))) "TraceTypeQuery1" false (Utilities|Array|MakeArray (Game|Player|GetPlayerPawn 0)) "ForDuration" false))
      (Utilities|IsValid _returnvalue_3
        (:Is%20Valid
          (Components|InstancedStaticMesh|AddInstance _returnvalue_3 (Math|Transform|MakeTransform (Math|Vector|MakeVector (Math|Float|SnapToGrid(Float) (.X (Math|Vector|BreakVector (.ImpactPoint (Collision|BreakHitResult _outhit)))) (Math|Conversions|ToFloat(Integer) _tile_size_2)) (Math|Float|SnapToGrid(Float) (.Y (Math|Vector|BreakVector (.ImpactPoint (Collision|BreakHitResult _outhit)))) (Math|Conversions|ToFloat(Integer) _tile_size_2)) (Math|Float|SnapToGrid(Float) (.Z (Math|Vector|BreakVector (.ImpactPoint (Collision|BreakHitResult _outhit)))) (Math|Conversions|ToFloat(Integer) _tile_size_2)))) false)))
      (else
        (bind _outhit_2 (Collision|LineTraceByChannel _returnvalue (+ _returnvalue (* (Math|Vector|GetForwardVector _firstpersoncamara) (Variables|Default|Get1000))) "TraceTypeQuery1" false (Utilities|Array|MakeArray (Game|Player|GetPlayerPawn 0)) "ForDuration" false))
        (Development|PrintString (Utilities|GetDisplayName (.HitActor (Collision|BreakHitResult _outhit_2))))
        (Development|PrintString (Utilities|String|ToString(Vector) (Transformation|GetActorLocation (Game|GetPlayerCharacter 0))))
        (Utilities|IsValid _returnvalue_4
          (:Is%20Valid
            (Components|InstancedStaticMesh|AddInstance _returnvalue_4 (Math|Transform|MakeTransform (Math|Vector|MakeVector (Math|Float|SnapToGrid(Float) (.X (Math|Vector|BreakVector (.ImpactPoint (Collision|BreakHitResult _outhit_2)))) (Math|Conversions|ToFloat(Integer) _tile_size)) (Math|Float|SnapToGrid(Float) (.Y (Math|Vector|BreakVector (.ImpactPoint (Collision|BreakHitResult _outhit_2)))) (Math|Conversions|ToFloat(Integer) _tile_size)) (Math|Float|SnapToGrid(Float) (.Z (Math|Vector|BreakVector (.ImpactPoint (Collision|BreakHitResult _outhit_2)))) (Math|Conversions|ToFloat(Integer) _tile_size)))) false)))))))

(fn ConstructionScript
  (bind _f2 (Variables|Default|GetF2))
  (bind _f3 (Variables|Default|GetF3))
  (bind _f1 (Variables|Default|GetF1))
  (bind _tile_size (Variables|Default|GetTile%20Size))
  (for _index (range 1 (Variables|Default|GetWidth))
    (for _index_2 (range 1 (Variables|Default|GetLength))
      (if (< (Math|Conversions|ToFloat(Integer) (* (Math|Float|Round (+ (* (Math|Trig|Sin(Degrees) (* _index _f1)) (Math|Trig|Sin(Degrees) (* _index_2 _f1)) (Variables|Default|GetH1)) (* (Math|Trig|Sin(Degrees) (* (* _index _f2) 0.7)) (Math|Trig|Sin(Degrees) (* _index_2 _f2)) (Variables|Default|GetH2)) (* (Math|Trig|Sin(Degrees) (* _index _f3)) (Math|Trig|Sin(Degrees) (* (* _index_2 _f3) 0.4)) (Variables|Default|GetH3)))) (Variables|Default|GetTile%20Size))) 0.0)
        (Components|InstancedStaticMesh|AddInstance (Variables|Default|GetDirt) (Math|Conversions|ToTransform(Vector) (Math|Vector|MakeVector (Math|Conversions|ToFloat(Integer) (* _index _tile_size)) (Math|Conversions|ToFloat(Integer) (* _index_2 _tile_size)) (Math|Conversions|ToFloat(Integer) (* (Math|Float|Round (+ (* (Math|Trig|Sin(Degrees) (* _index _f1)) (Math|Trig|Sin(Degrees) (* _index_2 _f1)) (Variables|Default|GetH1)) (* (Math|Trig|Sin(Degrees) (* (* _index _f2) 0.7)) (Math|Trig|Sin(Degrees) (* _index_2 _f2)) (Variables|Default|GetH2)) (* (Math|Trig|Sin(Degrees) (* _index _f3)) (Math|Trig|Sin(Degrees) (* (* _index_2 _f3) 0.4)) (Variables|Default|GetH3)))) (Variables|Default|GetTile%20Size))))) false)
        (else
          (Components|InstancedStaticMesh|AddInstance (Variables|Default|GetGrass) (Math|Conversions|ToTransform(Vector) (Math|Vector|MakeVector (Math|Conversions|ToFloat(Integer) (* _index _tile_size)) (Math|Conversions|ToFloat(Integer) (* _index_2 _tile_size)) (Math|Conversions|ToFloat(Integer) (* (Math|Float|Round (+ (* (Math|Trig|Sin(Degrees) (* _index _f1)) (Math|Trig|Sin(Degrees) (* _index_2 _f1)) (Variables|Default|GetH1)) (* (Math|Trig|Sin(Degrees) (* (* _index _f2) 0.7)) (Math|Trig|Sin(Degrees) (* _index_2 _f2)) (Variables|Default|GetH2)) (* (Math|Trig|Sin(Degrees) (* _index _f3)) (Math|Trig|Sin(Degrees) (* (* _index_2 _f3) 0.4)) (Variables|Default|GetH3)))) (Variables|Default|GetTile%20Size))))) false))))))